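; Falling-block platform that vanishes shortly after a character steps on it, then reappears.
; A Box overlap by an actor implementing Bp_inerface_karakter plays a Timeline that offsets the actor along X from the mesh's current world position.
; Delays chained from the Timeline update hide the mesh and disable collision, then restore both and stop the Timeline.
; The block never moves vertically.
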(event `self.Box.OnComponentBeginOverlap`
  (params (OverlappedComponent :type "PrimitiveComponent Object Reference") (OtherActor :type "Actor Object Reference") (OtherComp :type "PrimitiveComponent Object Reference") (OtherBodyIndex :type Integer) (bFromSweep :type Boolean) (SweepResult :type "HitResult Structure (by ref)"))
  (bind (_returnvalue_x _returnvalue_y _returnvalue_z) (`KismetMathLibrary.BreakVector` (`SceneComponent.K2_GetComponentLocation` (`self.StaticMesh`))))
  (if (`KismetSystemLibrary.DoesImplementInterface` OtherActor "/Game/bluprints/bp_inerface_karakter.bp_inerface_karakter_C")
    (bind (_direction _newtrack_0) (`Timeline|Timeline` :!label _label)
      (:`Update`
        (`self.K2_SetActorLocation` (`KismetMathLibrary.MakeVector` (+ (.y _newtrack_0) _returnvalue_x) _returnvalue_y _returnvalue_z))
        (`KismetSystemLibrary.Delay` 1.0)
        (`SceneComponent.SetVisibility` (`self.StaticMesh`) false false)
        (`PrimitiveComponent.SetCollisionEnabled` (`self.StaticMesh`) "NoCollision")
        (`KismetSystemLibrary.Delay` 2.0)
        (`SceneComponent.SetVisibility` (`self.StaticMesh`) true false)
        (`PrimitiveComponent.SetCollisionEnabled` (`self.StaticMesh`) "QueryAndPhysics")
        (goto _label :!via `Stop`)))))

(fn `UserConstructionScript`)