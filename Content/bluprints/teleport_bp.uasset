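; Two-way teleporter actor that moves the player character between two pads, Teleport1 and Teleport2.
; Overlapping either trigger box sends the first actor tagged "karakter_ref" to the opposite pad, offset along world X and raised slightly, then plays a slide sound attached to that destination.
; The overlapping actor is never checked, as the character interface tests are left unconnected, so any overlap triggers the teleport.
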(event `self.box1.OnComponentBeginOverlap`
  (params (OverlappedComponent :type "PrimitiveComponent Object Reference") (OtherActor :type "Actor Object Reference") (OtherComp :type "PrimitiveComponent Object Reference") (OtherBodyIndex :type Integer) (bFromSweep :type Boolean) (SweepResult :type "HitResult Structure (by ref)"))
  (bind (_returnvalue_x _returnvalue_y _returnvalue_z) (`KismetMathLibrary.BreakVector` (`SceneComponent.K2_GetComponentLocation` (`self.teleport2`))))
  (bind _outactors (`GameplayStatics.GetAllActorsWithTag` "karakter_ref"))
  (`self.K2_SetActorLocation` (`|GetArrayItem` _outactors) (`KismetMathLibrary.MakeVector` (+ _returnvalue_x 200.0) _returnvalue_y (+ _returnvalue_z 50.0)) false false)
  (`GameplayStatics.SpawnSoundAttached` "/Game/data/sound/slide_1_Cue.slide_1_Cue" (`self.teleport2`) "None" (0.0 0.0 0.0) (struct) "KeepRelativeOffset" false 1.0 1.0 0.0 null null))

(event `self.box2.OnComponentBeginOverlap`
  (params (OverlappedComponent :type "PrimitiveComponent Object Reference") (OtherActor :type "Actor Object Reference") (OtherComp :type "PrimitiveComponent Object Reference") (OtherBodyIndex :type Integer) (bFromSweep :type Boolean) (SweepResult :type "HitResult Structure (by ref)"))
  (bind (_returnvalue_x _returnvalue_y _returnvalue_z) (`KismetMathLibrary.BreakVector` (`SceneComponent.K2_GetComponentLocation` (`self.teleport1`))))
  (bind _outactors (`GameplayStatics.GetAllActorsWithTag` "karakter_ref"))
  (`self.K2_SetActorLocation` (`|GetArrayItem` _outactors) (`KismetMathLibrary.MakeVector` (+ _returnvalue_x 200.0) _returnvalue_y (+ _returnvalue_z 50.0)) false false)
  (`GameplayStatics.SpawnSoundAttached` "/Game/data/sound/slide_1_Cue.slide_1_Cue" (`self.teleport1`) "None" (0.0 0.0 0.0) (struct) "KeepRelativeOffset" false 1.0 1.0 0.0 null null))

(fn `UserConstructionScript`)