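; Coin pickup Blueprint that adds to the player character's coin count when collected.
; Overlapping the Sphere with a BP_KARAKTER adds the Para value to that character's Coin, plays a click sound at the mesh location and destroys the actor.
; The static mesh spins by a fixed local rotation step every Tick, not scaled by delta time.
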(event `self.Sphere.OnComponentBeginOverlap`
  (params (OverlappedComponent :type "PrimitiveComponent Object Reference") (OtherActor :type "Actor Object Reference") (OtherComp :type "PrimitiveComponent Object Reference") (OtherBodyIndex :type Integer) (bFromSweep :type Boolean) (SweepResult :type "HitResult Structure (by ref)"))
  (bind _asbp_karakter (cast `/Game/Isometric_World/Demo/Demo/Blueprints/BP_KARAKTER` OtherActor))
  (set `/Game/Isometric_World/Demo/Demo/Blueprints/BP_KARAKTER.coin` (+ (`self.para`) (`/Game/Isometric_World/Demo/Demo/Blueprints/BP_KARAKTER.coin` _asbp_karakter)) _asbp_karakter)
  (`GameplayStatics.SpawnSoundAtLocation` "/Engine/VREditor/Sounds/VR_click2.VR_click2" (`SceneComponent.K2_GetComponentLocation` (`self.StaticMesh`)) (struct) 1.0 1.0 0.0 null null)
  (`self.K2_DestroyActor`))

(event `self.ReceiveTick`
  (params (DeltaSeconds :type "Float (single-precision)"))
  (`SceneComponent.K2_AddLocalRotation` (`self.StaticMesh`) (struct :`Yaw` 1.0) false false))

(fn `UserConstructionScript`)